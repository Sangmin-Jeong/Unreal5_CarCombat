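; Player pawn Blueprint for a top-down, tank-style vehicle that drives, aims, fires, honks and can be destroyed.
; Axis input moves it with sweep and turns it only while moving, as Tick smoothly yaws the Top toward the cursor hit point, marked by a debug sphere.
; Construction raises MaxHealth and fills Health; damage depletes it, and at zero the pawn explodes, hides and loses input.
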(event `InputAxis|MoveForward`
  (params (AxisValue :type "Float (single-precision)"))
  ;[1 1 1] MoveForward * Speed * DeltaTime
  (set `self.IsMoving` (!= AxisValue 0.0))
  (`self.K2_AddActorLocalOffset` (`KismetMathLibrary.MakeVector` (* AxisValue (`self.Speed`) (`GameplayStatics.GetWorldDeltaSeconds`))) true)
  (if (`self.IsMoving`)
    (`GameplayStatics.PlaySound2D` "/Game/StarterContent/Audio/hitHurt.hitHurt" 5.0 1.0 0.0 null null)))

(event `self.ReceiveTick`
  (params (DeltaSeconds :type "Float (single-precision)"))
  (bind _top (`self.Top`))
  (bind _hitresult (`PlayerController.GetHitResultUnderCursorByChannel` (`GameplayStatics.GetPlayerController` 0) "TraceTypeQuery1" false))
  (bind (_returnvalue_roll _returnvalue_pitch _returnvalue_yaw) (`KismetMathLibrary.BreakRotator` (`KismetMathLibrary.RInterpTo` (`SceneComponent.K2_GetComponentRotation` _top) (`KismetMathLibrary.FindLookAtRotation` (`SceneComponent.K2_GetComponentLocation` _top) (`.ImpactPoint` (`GameplayStatics.BreakHitResult` _hitresult))) (`GameplayStatics.GetWorldDeltaSeconds`) 25.0)))
  ;[1 1 1] Cursor Location and Rotate Top
  (`|ExecutionSequence`
    (:`then_1`
      (`SceneComponent.K2_SetWorldRotation` _top (`KismetMathLibrary.MakeRotator` 0.0 0.0 _returnvalue_yaw) false false)
      (`KismetSystemLibrary.DrawDebugSphere` (`.ImpactPoint` (`GameplayStatics.BreakHitResult` _hitresult)) 25.0 12 (struct :`R` 1.0 :`A` 1.0) -1.0))))

(event `InputAxis|Turn`
  (params (AxisValue :type "Float (single-precision)"))
  ;[1 1 1] Turn * RotationRate * DeltaTime
  (if (`self.IsMoving`)
    (`self.K2_AddActorLocalRotation` (`KismetMathLibrary.MakeRotator` 0.0 0.0 (* AxisValue (`self.RotationRate`) (`GameplayStatics.GetWorldDeltaSeconds`))))))

(event `self.ReceiveBeginPlay`
  ;[1 1 1] Take Damage
  (add `self.OnTakeAnyDamage` (delegate `OnTakeAnyDamage_Event`)))

(event `InputAction|Fire`
  (params (Key :type "Key Structure"))
  (:`Pressed`
    (`self.Fire`)))

(event `OnTakeAnyDamage_Event` :!signature `self.OnTakeAnyDamage`
  (params (DamagedActor :type "Actor Object Reference") (Damage :type "Float (single-precision)") (DamageType :type "DamageType Object Reference") (InstigatedBy :type "Controller Object Reference") (DamageCauser :type "Actor Object Reference"))
  (bind _returnvalue (`GameplayStatics.GetPlayerPawn` 0))
  ;[1 1 1] Take Damage
  (`GameplayStatics.PlaySound2D` "/Game/StarterContent/Audio/hit.hit" 1.0 1.0 0.0 null null)
  (bind _output_get (set `self.Health` (- (`self.Health`) Damage)))
  (if (<= _output_get 0.0)
    (`self.Explode`)
    (cast `/Game/Blueprints/Player` _returnvalue)
    (`self.DisableInput` _returnvalue null)
    (`self.SetActorHiddenInGame` true)))

(event `InputAction|Honking`
  (params (Key :type "Key Structure"))
  (:`Pressed`
    (`GameplayStatics.PlaySound2D` "/Game/StarterContent/Audio/bicycle-horn-1.bicycle-horn-1" 1.0 1.0 0.0 null null)))

(fn `UserConstructionScript`
  (`parent.UserConstructionScript`)
  (bind _output_get (set `self.MaxHealth` (+ (`self.MaxHealth`) 300.0)))
  (set `self.Health` _output_get))