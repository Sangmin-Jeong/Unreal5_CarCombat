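; Base Blueprint for an actor with health that can shoot projectiles and explode, with no active event logic of its own.
; The construction script sets Health to MaxHealth.
; Fire spawns a scaled-up, self-owned BP_Projectile at ProjectileSpawnPoint with an explosion particle and sound.
; Explode plays only a larger explosion effect and collapse sound, without destroying the actor or changing Health.
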(event `self.ReceiveBeginPlay`)

(event `self.ReceiveTick`
  (params (DeltaSeconds :type "Float (single-precision)")))

(fn `Explode`
  (`GameplayStatics.SpawnEmitterAtLocation` "/Game/StarterContent/Particles/P_Explosion.P_Explosion" (`self.K2_GetActorLocation`) (struct) (3.0 3.0 3.0))
  (`GameplayStatics.PlaySound2D` "/Game/StarterContent/Audio/Collapse02.Collapse02" 3.0 1.0 0.0 null null))

(fn `Fire`
  (bind _projectile_spawn_point (`self.Projectile Spawn Point`))
  (bind _returnvalue (`SceneComponent.K2_GetComponentLocation` _projectile_spawn_point))
  (bind _returnvalue_2 (`SceneComponent.K2_GetComponentRotation` _projectile_spawn_point))
  (`|SpawnActorFromClass` "/Game/Blueprints/BP_Projectile.BP_Projectile_C" (`KismetMathLibrary.MakeTransform` _returnvalue _returnvalue_2 (2.0 2.0 2.0)) "Undefined" "OverrideRootScale" self null)
  (`GameplayStatics.SpawnEmitterAtLocation` "/Game/StarterContent/Particles/P_Explosion.P_Explosion" _returnvalue _returnvalue_2)
  (`GameplayStatics.PlaySound2D` "/Game/StarterContent/Audio/Explosion01.Explosion01" 1.0 1.0 0.0 null null))

(fn `UserConstructionScript`
  (set `self.Health` (`self.MaxHealth`)))