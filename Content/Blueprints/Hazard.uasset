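; Hazard actor that deals repeated damage to the Player while it overlaps the hazard's capsule.
; Capsule overlap sets an On flag, plays a hit sound and subtracts Health, then loops back after a one-second Delay while On holds.
; Actor end overlap by the Player clears the flag.
; When the first player pawn's Health runs out, the overlapping Player explodes, loses input and is hidden.
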(event `self.Capsule1.OnComponentBeginOverlap`
  (params (OverlappedComponent :type "PrimitiveComponent Object Reference") (OtherActor :type "Actor Object Reference") (OtherComp :type "PrimitiveComponent Object Reference") (OtherBodyIndex :type Integer) (bFromSweep :type Boolean) (SweepResult :type "HitResult Structure (by ref)"))
  (bind _asplayer (cast `/Game/Blueprints/Player` OtherActor :!label _label))
  (`GameplayStatics.PlaySound2D` "/Game/StarterContent/Audio/hit.hit" 1.0 1.0 0.0 null null)
  (set `self.On` true)
  (set `/Game/Blueprints/Base.Health` (- (`/Game/Blueprints/Base.Health` _asplayer) 21.0) _asplayer)
  (`KismetSystemLibrary.Delay` 1.0)
  (bind _asplayer_2 (cast `/Game/Blueprints/Player` (`GameplayStatics.GetPlayerPawn` 0)))
  (if (<= (`/Game/Blueprints/Base.Health` _asplayer_2) 0.0)
    (`/Game/Blueprints/Base.Explode` _asplayer)
    (`self.DisableInput` _asplayer (`GameplayStatics.GetPlayerController` 0))
    (`self.SetActorHiddenInGame` _asplayer true)
    (elif (`self.On`)
      (goto _label))))

(event `self.ReceiveActorEndOverlap`
  (params (OtherActor :type "Actor Object Reference"))
  (cast `/Game/Blueprints/Player` OtherActor)
  (set `self.On` false))

(fn `UserConstructionScript`)