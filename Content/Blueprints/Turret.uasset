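; Turret actor that tracks and fires at the player within range, and can be destroyed by damage.
; Tick runs a two-second fire countdown that calls Fire if the player is in range, and smoothly turns the Top component's yaw toward them.
; Range and aim checks look up the player by actor class on each call.
; Any damage plays a hit sound and lowers Health, calling Explode and destroying the actor at zero.
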(event `self.ReceiveBeginPlay`
  (`parent.ReceiveBeginPlay`)
  ;[1 1 1] Take Damage
  (add `self.OnTakeAnyDamage` (delegate `OnTakeDamage`)))

(event `OnTakeDamage` :!signature `self.OnTakeAnyDamage`
  (params (DamagedActor :type "Actor Object Reference") (Damage :type "Float (single-precision)") (DamageType :type "DamageType Object Reference") (InstigatedBy :type "Controller Object Reference") (DamageCauser :type "Actor Object Reference"))
  ;[1 1 1] Take Damage
  (`GameplayStatics.PlaySound2D` "/Game/StarterContent/Audio/hit.hit" 1.0 1.0 0.0 null null)
  (bind _output_get (set `self.Health` (- (`self.Health`) Damage)))
  (if (<= _output_get 0.0)
    (`self.Explode`)
    (`self.K2_DestroyActor`)))

(event `self.ReceiveTick`
  (params (DeltaSeconds :type "Float (single-precision)"))
  (`parent.ReceiveTick` DeltaSeconds)
  ;[1 1 1] In Fire Range, Rotation and Firing
  (bind _output_get (set `self.FireRate` (- (`self.FireRate`) DeltaSeconds)))
  (`self.CheckFire` (<= (`KismetMathLibrary.FCeil` _output_get) 0))
  (bind _newparam (`self.InFireRange`))
  (if _newparam
    (`self.Rotation`)))

(fn `CheckFire`
  (params (NewParam :type Boolean))
  (if NewParam
    (set `self.FireRate` 2.0)
    (bind _newparam (`self.InFireRange`))
    (if _newparam
      (`self.Fire`))))

(fn `InFireRange`
  (returns (NewParam :type Boolean))
  (locals (NewLocalVar_0 :type "Actor Class Reference"))
  (bind _asactor (castclass `Actor` "/Game/Blueprints/Player.Player_C"))
  (bind _returnvalue (`GameplayStatics.GetActorOfClass` _asactor))
  (return (<= (`KismetMathLibrary.Vector_Distance` (`self.K2_GetActorLocation`) (`self.K2_GetActorLocation` _returnvalue)) (`self.FireRange`))))

(fn `Rotation`
  (bind _top (`self.Top`))
  (bind _asactor (castclass `Actor` "/Game/Blueprints/Player.Player_C"))
  (bind _returnvalue (`GameplayStatics.GetActorOfClass` _asactor))
  (bind (_returnvalue_roll _returnvalue_pitch _returnvalue_yaw) (`KismetMathLibrary.BreakRotator` (`KismetMathLibrary.RInterpTo` (`SceneComponent.K2_GetComponentRotation` _top) (`KismetMathLibrary.FindLookAtRotation` (`SceneComponent.K2_GetComponentLocation` _top) (`self.K2_GetActorLocation` _returnvalue)) (`GameplayStatics.GetWorldDeltaSeconds`) 25.0)))
  (`SceneComponent.K2_SetWorldRotation` _top (`KismetMathLibrary.MakeRotator` 0.0 0.0 _returnvalue_yaw) false false))

(fn `UserConstructionScript`
  (`parent.UserConstructionScript`))