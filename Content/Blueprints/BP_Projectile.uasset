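; Projectile actor that damages the Player or Turret it hits and destroys itself on any hit.
; BeginPlay looks up a single Player and Turret actor by class and stores both references.
; On hit, it checks the other actor's class, prints a colored debug message and applies damage, crediting the opposite side's instigator controller rather than tracking who fired it.
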(event `self.ReceiveBeginPlay`
  (bind _returnvalue (`GameplayStatics.GetActorOfClass` "/Game/Blueprints/Player.Player_C"))
  (set `self.Player` _returnvalue)
  (bind _returnvalue_2 (`GameplayStatics.GetActorOfClass` "/Game/Blueprints/Turret.Turret_C"))
  (set `self.Turret` _returnvalue_2))

(event `self.ReceiveHit`
  (params (MyComp :type "PrimitiveComponent Object Reference") (Other :type "Actor Object Reference") (OtherComp :type "PrimitiveComponent Object Reference") (bSelfMoved :type Boolean) (HitLocation :type "Vector Structure") (HitNormal :type "Vector Structure") (NormalImpulse :type "Vector Structure") (Hit :type "HitResult Structure (by ref)"))
  (bind _returnvalue (`GameplayStatics.GetObjectClass` Other))
  (`self.K2_DestroyActor`)
  (if (== _returnvalue "/Game/Blueprints/Player.Player_C")
    (`KismetSystemLibrary.PrintString` "Player Hit!" true false (struct :`R` 1.0 :`B` 0.173289 :`A` 1.0))
    (`GameplayStatics.ApplyDamage` Other (`self.Damage`) (`self.GetInstigatorController` (`self.Turret`)) self "/Script/Engine.DamageType")
    (elif (== _returnvalue "/Game/Blueprints/Turret.Turret_C")
      (`KismetSystemLibrary.PrintString` "Turret Hit!" true false (struct :`G` 0.176688 :`B` 1.0 :`A` 1.0))
      (`GameplayStatics.ApplyDamage` Other (`self.Damage`) (`self.GetInstigatorController` (`self.Player`)) self "/Script/Engine.DamageType"))))

(fn `UserConstructionScript`)